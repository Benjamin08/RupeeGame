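; BP_RupeeTarget is a damageable rupee target actor for the BlockBreaker game.
; It starts immune to damage, and Enable and Disable events toggle both damageability and actor visibility.
; AnyDamage feeds TakeDamage, which lowers clamped Health and, at zero, hides the rupee mesh and turns off its collision instead of destroying the actor.
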(event `self.ReceiveBeginPlay`
  (set `self.bCanBeDamaged` false))

(event `Enable`
  (set `self.bCanBeDamaged` true)
  (`self.SetActorHiddenInGame` false))

(event `Disable`
  (set `self.bCanBeDamaged` false)
  (`self.SetActorHiddenInGame` true))

(event `self.ReceiveAnyDamage`
  (params (Damage :type "Float (single-precision)") (DamageType :type "DamageType Object Reference") (InstigatedBy :type "Controller Object Reference") (DamageCauser :type "Actor Object Reference"))
  (`self.Take Damage` Damage))

(fn `Take Damage`
  (params (Damage :type "Float (double-precision)"))
  (bind _rupeemesh (`self.RupeeMesh`))
  (bind _output_get (set `self.Health` (`KismetMathLibrary.FClamp` (- (`self.Health`) Damage) 0.0 10.0)))
  (if (== _output_get 0.0)
    (`SceneComponent.SetVisibility` _rupeemesh false false)
    (`PrimitiveComponent.SetCollisionEnabled` _rupeemesh "NoCollision")))

(fn `UserConstructionScript`)