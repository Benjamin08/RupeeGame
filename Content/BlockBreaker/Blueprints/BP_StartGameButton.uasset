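; BP_StartGameButton is a block-breaker start button actor that runs a round-start countdown.
; Tick passes through a one-second Delay into StartRound, which decrements and prints TimerValue once per second.
; When the timer runs out, it clears Shot and sets MoveRupees, though nothing in this graph reads either flag.
; Taking any damage calls ShotFunction, which only prints a debug string and does not affect the countdown.
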(event `self.ReceiveTick`
  (params (DeltaSeconds :type "Float (single-precision)"))
  (`KismetSystemLibrary.Delay` 1.0)
  (`self.StartRound`))

(event `self.ReceiveAnyDamage`
  (params (Damage :type "Float (single-precision)") (DamageType :type "DamageType Object Reference") (InstigatedBy :type "Controller Object Reference") (DamageCauser :type "Actor Object Reference"))
  (`self.ShotFunction`))

(fn `ShotFunction`
  (`KismetSystemLibrary.PrintString` "Shot Function"))

(fn `StartRound`
  (if (> (`self.TimerValue`) 0)
    (set `self.TimerValue` (- (`self.TimerValue`) 1))
    (`KismetSystemLibrary.PrintString` (`KismetStringLibrary.Conv_IntToString` (`self.TimerValue`)))
    (if (<= (`self.TimerValue`) 0)
      (set `self.Shot` false)
      (set `self.MoveRupees` true))))

(fn `UserConstructionScript`)