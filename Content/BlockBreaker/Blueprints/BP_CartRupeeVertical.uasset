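; BP_CartRupeeVertical is a destructible BlockBreaker cart that travels along the spline of a referenced track actor.
; It moves on BeginPlay if already active, or when SetActive is called.
; The CartMover timeline, scaled by Duration and begun at CartStartOffset, maps its alpha to distance along the spline.
; Damage lowers clamped Health, and at zero the mesh is hidden and loses collision without destroying the actor.
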(event `self.ReceiveBeginPlay`
  (if (`self.Active Cart`)
    (`self.MoveCart`)))

(event `MoveCart`
  (`TimelineComponent.SetPlayRate` (`self.CartMover`) (/ 1.0 (`self.Duration`)))
  (`TimelineComponent.SetNewTime` (`self.CartMover`) (`self.Cart Start Offset`))
  (bind (_direction _alpha) (`Timeline|CartMover`)
    (:`Update`
      (set `self.Alpha` _alpha)
      (`self.K2_SetActorLocationAndRotation` (`SplineComponent.GetLocationAtDistanceAlongSpline` (`/Game/BlockBreaker/Blueprints/BP_SplineTrack1.UsefulSpline` (`self.Track Ref`)) (`KismetMathLibrary.Lerp` 0.0 (`SplineComponent.GetSplineLength` (`/Game/BlockBreaker/Blueprints/BP_SplineTrack1.UsefulSpline` (`self.Track Ref`))) (`self.Alpha`)) "World")))))

(event `self.ReceiveAnyDamage`
  (params (Damage :type "Float (single-precision)") (DamageType :type "DamageType Object Reference") (InstigatedBy :type "Controller Object Reference") (DamageCauser :type "Actor Object Reference"))
  (`self.Take Damage` Damage))

(event `SetActive`
  (set `self.Active Cart` true)
  (`self.MoveCart`))

(fn `Take Damage`
  (params (Damage :type "Float (double-precision)"))
  (bind _cartmesh (`self.CartMesh`))
  (bind _output_get (set `self.Health` (`KismetMathLibrary.FClamp` (- (`self.Health`) Damage) 0.0 10.0)))
  (if (== _output_get 0.0)
    (`SceneComponent.SetVisibility` _cartmesh false false)
    (`PrimitiveComponent.SetCollisionEnabled` _cartmesh "NoCollision")))

(fn `UserConstructionScript`)